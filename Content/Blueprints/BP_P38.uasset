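; BP_P38 is a player-flown P-38 plane that moves continuously forward and fires rockets.
; BeginPlay adds the IMC_FlightMode Enhanced Input context, whose actions adjust a clamped velocity, pitch (optionally inverted) and roll through local rotations.
; Tick spins both propellers at a fixed per-frame rate and offsets the actor along its forward vector by that velocity, without delta-time scaling or sweep.
; The fire action spawns a BP_Rocket at the RocketLocation component.
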(event `self.ReceiveBeginPlay`
  (`EnhancedInputSubsystemInterface.AddMappingContext` (pcsubsystem `EnhancedInputLocalPlayerSubsystem` (`GameplayStatics.GetPlayerController` 0)) "/Game/Inputs/IMC_FlightMode.IMC_FlightMode" 0 (struct)))

(event `self.ReceiveTick`
  (params (DeltaSeconds :type "Float (single-precision)"))
  ;[1 1 1] Tick Flight Move and Propeller Rotate
  (`SceneComponent.K2_AddRelativeRotation` (`self.Propeller1`) (struct :`Roll` 10.0) false false)
  (`SceneComponent.K2_AddRelativeRotation` (`self.Propeller2`) (struct :`Roll` 10.0) false false)
  (`self.K2_AddActorWorldOffset` (* (`self.GetActorForwardVector`) (`self.Velocity`))))

(event `EnhancedInput|/Game/Inputs/IA_Accelerate`
  (params (ActionValue :type "Float (double-precision)") (ElapsedSeconds :type "Float (double-precision)") (TriggeredSeconds :type "Float (double-precision)") (InputAction :type "InputAction Object Reference" :default "/Game/Inputs/IA_Accelerate.IA_Accelerate"))
  ;[1 1 1] Set Accelerate
  (:`Triggered`
    (set `self.Velocity` (`KismetMathLibrary.FClamp` (+ ActionValue (`self.Velocity`)) (`self.MinSpeed`) (`self.MaxSpeed`)))))

(event `EnhancedInput|/Game/Inputs/IA_RotatePitch`
  (params (ActionValue :type "Float (double-precision)") (ElapsedSeconds :type "Float (double-precision)") (TriggeredSeconds :type "Float (double-precision)") (InputAction :type "InputAction Object Reference" :default "/Game/Inputs/IA_RotatePitch.IA_RotatePitch"))
  ;[1 1 1] Rotate Pitch
  (:`Triggered`
    (if (`self.IsInvertPitch`)
      (`self.K2_AddActorLocalRotation` (`KismetMathLibrary.MakeRotator` 0.0 ActionValue))
      (else
        (`self.K2_AddActorLocalRotation` (`KismetMathLibrary.MakeRotator` 0.0 (* ActionValue -1.0)))))))

(event `EnhancedInput|/Game/Inputs/IA_RotateRoll`
  (params (ActionValue :type "Float (double-precision)") (ElapsedSeconds :type "Float (double-precision)") (TriggeredSeconds :type "Float (double-precision)") (InputAction :type "InputAction Object Reference" :default "/Game/Inputs/IA_RotateRoll.IA_RotateRoll"))
  ;[1 1 1] Rotate Roll
  (:`Triggered`
    (`self.K2_AddActorLocalRotation` (`KismetMathLibrary.MakeRotator` ActionValue))))

(event `EnhancedInput|/Game/Inputs/IA_Fire`
  (params (ActionValue :type Boolean) (ElapsedSeconds :type "Float (double-precision)") (TriggeredSeconds :type "Float (double-precision)") (InputAction :type "InputAction Object Reference" :default "/Game/Inputs/IA_Fire.IA_Fire"))
  ;[1 1 1] Fire
  (:`Started`
    (`|SpawnActorFromClass` "/Game/Blueprints/BP_Rocket.BP_Rocket_C" (`SceneComponent.K2_GetComponentToWorld` (`self.RocketLocation`)) "Undefined" "MultiplyWithRoot" null null)))

(fn `UserConstructionScript`)